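; Gameplay ability that listens for health attribute changes on its owner's Ability System Component.
; On activation it starts a ListenForAttributeChange async task and stores it.
; Each change only prints the avatar's name and new value, gated by a DrawDebugs check.
; Ending the ability also ends the stored task if it is still valid.
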(event `self.K2_ActivateAbility`
  (bind (_asynctaskproxy _attribute _newvalue) (`GC_AttributeChangeTask.ListenForAttributeChange` (`self.GetAbilitySystemComponentFromActorInfo`) (struct :`AttributeName` "Health" :`Attribute` "/Script/GSCProject.GC_AttributeSet:Health" :`AttributeOwner` "/Script/CoreUObject.Class'/Script/GSCProject.GC_AttributeSet'"))
    (:`then`
      (set `self.AttributeChangeTask` _asynctaskproxy))
    (:`OnAttributeChanged`
      (`self.bDrawDebugs`
        (:`then`
          (`KismetSystemLibrary.PrintString` (`KismetStringLibrary.Concat_StrStr` "GA_GC_ListenForHealthChange for:" (`KismetSystemLibrary.GetDisplayName` (`self.GetAvatarActorFromActorInfo`)) "New Health Value:" (`KismetStringLibrary.Conv_DoubleToString` _newvalue))))
        (:`else`)))))

(event `self.K2_OnEndAbility`
  (params (bWasCancelled :type Boolean))
  (bind _attributechangetask (`self.AttributeChangeTask`)
    (:`then`
      (`GC_AttributeChangeTask.EndTask` _attributechangetask))
    (:`else`)))