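; Enemy gameplay ability that plays a directional hit reaction montage.
; On activation it waits for the HitReact gameplay event, then caches direction vectors from the event's instigator.
; It converts the avatar forward and to-instigator vectors into a direction name, used as the montage section to jump to.
; The ability never ends itself here, and debug prints are gated by DrawDebugs.
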(event `self.K2_ActivateAbility`
  (bind (_asynctaskproxy _payload) (`AbilityTask_WaitGameplayEvent.WaitGameplayEvent` (struct :`TagName` "GCTags.Events.Enemy.HitReact") null)
    (:`EventReceived`
      (`self.PrintDebugEventReceived` _payload)
      (`self.CacheHitDirectionVectors` (`.Instigator` (break `GameplayEventData` _payload)))
      (`|ExecutionSequence`
        (:`then_0`
          ;[0 0.2985 1] Cache Hit Direction Name
          (set `self.HitDirectionName` (`GC_BlueprintLibrary.GetHitDirectionName` (`GC_BlueprintLibrary.GetHitDirection` (`self.AvatarForward`) (`self.ToInstigator`))))
          ;[1 0 0.02401] Debug For Hit Direction
          (`self.bDrawDebugs`
            (:`then`
              (`KismetSystemLibrary.PrintString` (`KismetStringLibrary.Conv_NameToString` (`self.HitDirectionName`))))
            (:`else`)))
        (:`then_1`
          (`AbilityTask_PlayMontageAndWait.CreatePlayMontageAndWaitProxy` "None" (`self.HitReactMontage`)
            (:`then`
              (`self.MontageJumpToSection` (`self.HitDirectionName`)))))))))

(event `self.K2_OnEndAbility`
  (params (bWasCancelled :type Boolean)))

(fn `PrintDebugEventReceived`
  (params (GameplayEventData :type "GameplayEventData Structure"))
  (`self.bDrawDebugs`
    (:`then`
      (`KismetSystemLibrary.PrintString` (`KismetStringLibrary.Concat_StrStr` "GA_GC_HitReact Received Event From:" (`KismetSystemLibrary.GetDisplayName` (`.Instigator` (break `GameplayEventData` GameplayEventData)))) true true (struct :`R` 0.542035 :`B` 0.626736 :`A` 1.0)))
    (:`else`)))